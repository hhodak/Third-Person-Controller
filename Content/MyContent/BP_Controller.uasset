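; BP_Controller is a player controller Blueprint that turns input bindings into movement, look, jump and crouch for player 0's pawn.
; Move axes add movement input along forward and right vectors built from control-rotation yaw only, so pitch does not affect direction.
; Turn axes add controller pitch and yaw input, while Jump and Crouch actions start on press and stop on release through the player character.
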(event `InputAction|Jump`
  (params (Key :type "Key Structure"))
  (bind _returnvalue (`GameplayStatics.GetPlayerCharacter` 0))
  ;[1 1 1] Jumping
  (:`Pressed`
    (`Character.Jump` _returnvalue))
  (:`Released`
    (`Character.StopJumping` _returnvalue)))

(event `InputAxis|TurnUpDown`
  (params (AxisValue :type "Float (single-precision)"))
  ;[1 1 1] Mouse Controls
  (`Pawn.AddControllerPitchInput` (`GameplayStatics.GetPlayerPawn` 0) AxisValue))

(event `InputAxis|TurnRightLeft`
  (params (AxisValue :type "Float (single-precision)"))
  ;[1 1 1] Mouse Controls
  (`Pawn.AddControllerYawInput` (`GameplayStatics.GetPlayerPawn` 0) AxisValue))

(event `InputAction|Crouch`
  (params (Key :type "Key Structure"))
  (bind _returnvalue (`GameplayStatics.GetPlayerCharacter` 0))
  ;[1 1 1] Crouching
  (:`Pressed`
    (`Character.Crouch` _returnvalue))
  (:`Released`
    (`Character.UnCrouch` _returnvalue)))

(event `InputAxis|ForwardBackward`
  (params (AxisValue :type "Float (single-precision)"))
  (`Pawn.AddMovementInput` (`GameplayStatics.GetPlayerPawn` 0) (`KismetMathLibrary.GetForwardVector` (`KismetMathLibrary.MakeRotator` 0.0 0.0 (.yaw (`self.GetControlRotation`)))) AxisValue false))

(event `InputAxis|RightLeft`
  (params (AxisValue :type "Float (single-precision)"))
  (`Pawn.AddMovementInput` (`GameplayStatics.GetPlayerPawn` 0) (`KismetMathLibrary.GetRightVector` (`KismetMathLibrary.MakeRotator` 0.0 0.0 (.yaw (`self.GetControlRotation`)))) AxisValue false))

(fn `UserConstructionScript`)